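; Tank actor that pushes its physics Body forward or backward based on where a Target_BP actor lies.
; BeginPlay caches the location of the first Target_BP found, so later target movement is not tracked.
; Each Tick, the dot product of Body forward and target direction becomes a signed thrust, printed for debugging.
; That thrust scales a forward-axis force with mass, Acceleration and delta time, with no steering.
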(event Collision|EventActorBeginOverlap
  (params (OtherActor :type Actor%20Object%20Reference)))

(event EventBeginPlay
  ;[1 1 1] Getting the Target Blueprint
  (bind _outactors (Actor|GetAllActorsOfClass "/Game/Target/Target_BP.Target_BP_C"))
  (Variables|Default|SetTarget_BP (Utilities|Array|Get(acopy) _outactors))
  ;[1 1 1] Getting the Target Location
  (Variables|Default|SetTargetLocation (Transformation|GetActorLocation (Variables|Default|GetTarget_BP))))

(event EventTick
  (params (DeltaSeconds :type Float%20%28single-precision%29))
  (bind _body (Variables|Default|GetBody))
  (Variables|Default|SetDeltaTime DeltaSeconds)
  ;[1 1 1] Getting the target direction according to tank
  (Variables|Default|SetTargetDirection (Math|Vector|Normalize (- (Variables|Default|GetTargetLocation) (Transformation|GetActorLocation))))
  ;[1 1 1] Calculating the Thrust value
  (bind _output_get (Variables|Default|SetThrust (Math|Vector|DotProduct (Math|Vector|GetForwardVector (Variables|Default|GetBody)) (Variables|Default|GetTargetDirection))))
  (Development|PrintString (Utilities|String|ToString(Float) _output_get))
  ;[1 1 1] Calculating The Tank Movement Force
  (bind _output_get_2 (Variables|Default|SetForce (* (Math|Vector|GetForwardVector _body) (* (Physics|GetMass _body) (Variables|Default|GetAcceleration) (Variables|Default|GetThrust) (Variables|Default|GetDeltaTime)))))
  (Physics|AddForce (Variables|Default|GetBody) _output_get_2 "None" false))

(fn ConstructionScript)