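; Missile actor that pushes its physics body forward when play begins.
; BeginPlay makes a single AddForceAtLocation call along the body's forward vector at the Back component's location, scaled by mass and half the Acceleration value.
; No per-tick thrust or overlap response is active, and leftover Front1 and DeltaTime nodes are unconnected.
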(event Collision|EventActorBeginOverlap
  (params (OtherActor :type Actor%20Object%20Reference)))

(event EventBeginPlay
  (Class|PrimitiveComponent|AddForceatLocation (Variables|Default|GetMissileBody) (* (Math|Vector|GetForwardVector (Variables|Default|GetMissileBody)) (* (Physics|GetMass (Variables|Default|GetMissileBody)) (Variables|Default|GetAcceleration) 0.5)) (Transformation|GetSocketLocation (Variables|Default|GetBack) "None") "None"))

(fn ConstructionScript)